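; Walker spawner Blueprint that spawns automated pedestrian characters with varied walking speeds.
; SpawnWalker overrides no event logic; it picks a class from AutomatedClasses using the base class's random engine and spawns it at the given transform.
; Valid walkers orient to movement and get a max walk speed drawn from a clamped normal distribution.
; Using that shared engine for both class and speed keeps randomness in one source.
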(event `self.ReceiveBeginPlay`)

(fn `SpawnWalker`
  (params (SpawnTransform :type "Transform Structure (by ref)"))
  (returns (SpawnedCharacter :type "Character Object Reference"))
  ;[1 1 1] If you need a random number, request the random engine stored in the base class.
  (bind _returnvalue (`self.GetRandomEngine`))
  (bind _item (`self.PickOneFromArray` _returnvalue (`self.AutomatedClasses`)))
  (bind _returnvalue_2 (`|SpawnActorFromClass` _item SpawnTransform "Undefined" "OverrideRootScale" null _returnvalue null))
  (if (`KismetSystemLibrary.IsValid` _returnvalue_2)
    (bind _charactermovement (`Character.CharacterMovement` _returnvalue_2))
    (set `CharacterMovementComponent.bOrientRotationToMovement` true _charactermovement)
    (bind _returnvalue_3 (`RandomEngine.GetNormalDistribution` _returnvalue 120.0 50.0))
    (set `CharacterMovementComponent.MaxWalkSpeed` (`KismetMathLibrary.FClamp` _returnvalue_3 71.0 213.0) _charactermovement)
    (return _returnvalue_2)
    (else
      (return _returnvalue_2))))

(fn `UserConstructionScript`)